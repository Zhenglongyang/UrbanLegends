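; Level 2 wireboard puzzle actor where clicking a wire and then a connector makes a connection.
; Clicks on any of three wires or their colliders store that wire as FirstClick and set Clicked.
; Only Wire2 to Connector0 connects, swapping the loose wire for a connected mesh and lighting the main LED and a switchboard light.
; Other connectors are stubs, and the light-setting helper function is unused, with its On/Off branch disconnected.
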(event OnClicked(Wire0)
  (params (TouchedComponent :type Primitive%20Component%20Object%20Reference) (ButtonPressed :type Key%20Structure))
  (Development|PrintString "Clicked on Wire 1" true true "(R=0.000000,G=0.660000,B=1.000000,A=1.000000)" (Variables|Default|GetTextDuration))
  (Variables|Default|SetFirstClick (Variables|Default|GetWire0))
  (Variables|Default|SetClicked true))

(event OnClicked(ColliderWire0)
  (params (TouchedComponent :type Primitive%20Component%20Object%20Reference) (ButtonPressed :type Key%20Structure))
  (Development|PrintString "Clicked on Wire 1" true true "(R=0.000000,G=0.660000,B=1.000000,A=1.000000)" (Variables|Default|GetTextDuration))
  (Variables|Default|SetFirstClick (Variables|Default|GetWire0))
  (Variables|Default|SetClicked true))

(event OnClicked(Connector4)
  (params (TouchedComponent :type Primitive%20Component%20Object%20Reference) (ButtonPressed :type Key%20Structure)))

(event OnClicked(Connector5)
  (params (TouchedComponent :type Primitive%20Component%20Object%20Reference) (ButtonPressed :type Key%20Structure)))

(event OnClicked(Wire2)
  (params (TouchedComponent :type Primitive%20Component%20Object%20Reference) (ButtonPressed :type Key%20Structure))
  (Development|PrintString "Clicked on Wire 3" true true "(R=0.000000,G=0.660000,B=1.000000,A=1.000000)" (Variables|Default|GetTextDuration))
  (Variables|Default|SetFirstClick (Variables|Default|GetWire2))
  (Variables|Default|SetClicked true))

(event OnClicked(ColliderWire2)
  (params (TouchedComponent :type Primitive%20Component%20Object%20Reference) (ButtonPressed :type Key%20Structure))
  (Development|PrintString "Clicked on Wire 3" true true "(R=0.000000,G=0.660000,B=1.000000,A=1.000000)" (Variables|Default|GetTextDuration))
  (Variables|Default|SetFirstClick (Variables|Default|GetWire2))
  (Variables|Default|SetClicked true))

(event OnClicked(Wire1)
  (params (TouchedComponent :type Primitive%20Component%20Object%20Reference) (ButtonPressed :type Key%20Structure))
  (Development|PrintString "Clicked on Wire 2" true true "(R=0.000000,G=0.660000,B=1.000000,A=1.000000)" (Variables|Default|GetTextDuration))
  (Variables|Default|SetFirstClick (Variables|Default|GetWire1))
  (Variables|Default|SetClicked true))

(event OnClicked(ColliderWire1)
  (params (TouchedComponent :type Primitive%20Component%20Object%20Reference) (ButtonPressed :type Key%20Structure))
  (Development|PrintString "Clicked on Wire 2" true true "(R=0.000000,G=0.660000,B=1.000000,A=1.000000)" (Variables|Default|GetTextDuration))
  (Variables|Default|SetFirstClick (Variables|Default|GetWire1))
  (Variables|Default|SetClicked true))

(event OnClicked(Connector0)
  (params (TouchedComponent :type Primitive%20Component%20Object%20Reference) (ButtonPressed :type Key%20Structure))
  (Development|PrintString "Clicked COnnector 0")
  (if (Variables|Default|GetClicked)
    (if (and (== (Variables|Default|GetFirstClick) (Variables|Default|GetWire2)) (== TouchedComponent (Variables|Default|GetConnector0)))
      (Rendering|SetVisibility (Variables|Default|GetWire2) false true)
      (Rendering|SetVisibility (Variables|Default|Getwires_Cylinder_005) true true)
      (Rendering|Material|SetMaterial (Variables|Default|GetMainLED) 0 "/Game/Assets/WireBoard/Material/LED_ON.LED_ON")
      (Rendering|Material|SetMaterial (Variables|Default|GetSwichboard_Lights) 1 "/Game/Assets/WireBoard/Material/LED_ON.LED_ON"))))

(event OnClicked(Connector1)
  (params (TouchedComponent :type Primitive%20Component%20Object%20Reference) (ButtonPressed :type Key%20Structure)))

(event OnClicked(Connector2)
  (params (TouchedComponent :type Primitive%20Component%20Object%20Reference) (ButtonPressed :type Key%20Structure)))

(event OnClicked(Connector3)
  (params (TouchedComponent :type Primitive%20Component%20Object%20Reference) (ButtonPressed :type Key%20Structure))
  (Development|PrintString "Clicked COnnector 0"))

(event EventBeginPlay)

(event Collision|EventActorBeginOverlap
  (params (OtherActor :type Actor%20Object%20Reference)))

(event EventTick
  (params (DeltaSeconds :type Float%20%28single-precision%29)))

(fn ConstructionScript)

(fn NewFunction0
  (params (Light%20number :type Integer) (On :type Boolean))
  (Rendering|Material|SetMaterial (Variables|Default|GetSwichboard_Lights) Light%20number "/Game/Assets/WireBoard/Material/LED_ON.LED_ON"))