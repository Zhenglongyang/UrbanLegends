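; Camera actor that follows one of a list of target actors, letting the player cycle between them with the Q key.
; On BeginPlay it enables input for player 0, and Q advances the target index, wrapping to the first after the last.
; Each tick, LerpToTransform teleports the root halfway toward the current target's transform, giving a smoothed but frame-rate-dependent blend.
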(event EventBeginPlay
  (Input|EnableInput (Game|GetPlayerController 0)))

(event Collision|EventActorBeginOverlap
  (params (OtherActor :type Actor%20Object%20Reference)))

(event EventTick
  (params (DeltaSeconds :type Float%20%28single-precision%29))
  (CallFunction|LerptoTransform (Transformation|GetActorTransform (Utilities|Array|Get(acopy) (Variables|Default|GetTargets) (Variables|Default|GetcurrentTarget)))))

(event Input|KeyboardEvents|Q
  (params (Key :type Key%20Structure))
  (:Pressed
    (if (>= (Variables|Default|GetcurrentTarget) (Utilities|Array|LastIndex (Variables|Default|GetTargets)))
      (Variables|Default|SetcurrentTarget 0)
      (else
        (Variables|Default|SetcurrentTarget (+ (Variables|Default|GetcurrentTarget) 1))))))

(fn ConstructionScript)

(fn LerptoTransform
  (params (NewTransform :type Transform))
  (bind _scenecomponent (Variables|Default|GetSceneComponent))
  (Transformation|SetWorldTransform _scenecomponent (Math|Interpolation|Ease "Linear" 0.5 (Transformation|GetWorldTransform _scenecomponent) NewTransform) false true))