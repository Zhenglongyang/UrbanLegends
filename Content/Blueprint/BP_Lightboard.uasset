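; Lightboard memory puzzle that flashes a colored light sequence, then takes answers on nine buttons.
; BeginPlay decodes Level.Sequence cell-color pairs into SolutionString: green adds the cell, blue doubles it, yellow copies the second-to-last solution entry, red adds nothing.
; EnableTimer starts a looping timer that plays each pair, then enables input.
; Correct clicks advance StringIndex and light up, wrong ones are ignored, and completion only prints a victory message.
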(event OnClicked(Button1)
  (params (TouchedComponent :type Primitive%20Component%20Object%20Reference) (ButtonPressed :type Key%20Structure))
  (CallFunction|ProcessClick 1))

(event OnClicked(Button2)
  (params (TouchedComponent :type Primitive%20Component%20Object%20Reference) (ButtonPressed :type Key%20Structure))
  (CallFunction|ProcessClick 2))

(event OnClicked(Button3)
  (params (TouchedComponent :type Primitive%20Component%20Object%20Reference) (ButtonPressed :type Key%20Structure))
  (CallFunction|ProcessClick 3))

(event OnClicked(Button4)
  (params (TouchedComponent :type Primitive%20Component%20Object%20Reference) (ButtonPressed :type Key%20Structure))
  (CallFunction|ProcessClick 4))

(event OnClicked(Button5)
  (params (TouchedComponent :type Primitive%20Component%20Object%20Reference) (ButtonPressed :type Key%20Structure))
  (CallFunction|ProcessClick 5))

(event OnClicked(Button6)
  (params (TouchedComponent :type Primitive%20Component%20Object%20Reference) (ButtonPressed :type Key%20Structure))
  (CallFunction|ProcessClick 6))

(event OnClicked(Button7)
  (params (TouchedComponent :type Primitive%20Component%20Object%20Reference) (ButtonPressed :type Key%20Structure))
  (CallFunction|ProcessClick 7))

(event OnClicked(Button8)
  (params (TouchedComponent :type Primitive%20Component%20Object%20Reference) (ButtonPressed :type Key%20Structure))
  (CallFunction|ProcessClick 8))

(event OnClicked(Button9)
  (params (TouchedComponent :type Primitive%20Component%20Object%20Reference) (ButtonPressed :type Key%20Structure))
  (CallFunction|ProcessClick 9))

(event Custom|GoThroughSequence
  (CallFunction|GoThroughSequenceFct))

(event Custom|EnableTimer
  (bind _returnvalue (Utilities|Time|SetTimerbyEvent (delegate Custom|GoThroughSequence) (.Period (Utilities|Struct|BreakSTR_LightboardLevel (Variables|Default|GetLevel))) true))
  (Variables|Default|SetTimerHandle _returnvalue))

(event EventBeginPlay
  (for (_array_element _array_index) (Utilities|String|GetCharacterArrayfromString (.Sequence (Utilities|Struct|BreakSTR_LightboardLevel (Variables|Default|GetLevel))))
    (if (== (Math|Integer|%(Integer) _array_index 2) 0)
      (Variables|Default|Setcell _array_element)
      (elif (Utilities|Enum|Equal(Enum) _array_element "g")
        (Variables|Default|SetSolutionString (Utilities|String|Append (Variables|Default|GetSolutionString) (Variables|Default|Getcell)))
        (elif (Utilities|Enum|Equal(Enum) _array_element "b")
          (Variables|Default|SetSolutionString (Utilities|String|Append (Variables|Default|GetSolutionString) (Utilities|String|Append (Variables|Default|Getcell) (Variables|Default|Getcell))))
          (elif (Utilities|Enum|Equal(Enum) _array_element "y")
            (Variables|Default|SetSolutionString (Utilities|String|Append (Variables|Default|GetSolutionString) (Utilities|Array|Get(acopy) (Utilities|String|GetCharacterArrayfromString (Variables|Default|GetSolutionString)) (- (Utilities|Array|LastIndex (Utilities|String|GetCharacterArrayfromString (Variables|Default|GetSolutionString))) 1)))))))))
  (Development|PrintString (Variables|Default|GetSolutionString) true true "(R=0.000000,G=0.660000,B=1.000000,A=1.000000)" 2e+02)
  (CallFunction|TurnLightsOff))

(event Collision|EventActorBeginOverlap
  (params (OtherActor :type Actor%20Object%20Reference)))

(event EventTick
  (params (DeltaSeconds :type Float%20%28single-precision%29)))

(fn ConstructionScript)

(fn SuccessfulClick
  (params (LightIndex :type Integer))
  (CallFunction|TurnLighton LightIndex "/Game/Assets/WireBoard/Material/LED_ON.LED_ON")
  (if (== (Variables|Default|GetStringIndex) (Utilities|String|Len (Variables|Default|GetSolutionString)))
    (Development|PrintString "SWEET, SWEET, VICTORY")))

(fn ProcessClick
  (params (LightIndex :type Integer))
  (bind _returnvalue (Utilities|String|ToString(Integer) LightIndex))
  (bind _returnvalue_2 (Utilities|String|MakeLiteralString _returnvalue))
  (if (Variables|Default|GetbAwaitingInput)
    (if (Utilities|Enum|Equal(Enum) (Utilities|Array|Get(acopy) (Utilities|String|GetCharacterArrayfromString (Variables|Default|GetSolutionString)) (Variables|Default|GetStringIndex)) _returnvalue_2)
      (bind _result (Math|Integer|IncrementInt (Variables|Default|GetStringIndex))
        (:%20%20
          (Variables|Default|SetStringIndex _result)
          (CallFunction|SuccessfulClick (Math|Conversions|ToInteger(Byte) _returnvalue_2)))))))

(fn TurnLightsOff
  (bind _lights (Variables|Default|GetLights))
  (for _index (range 0 11)
    (if (== _index 0)
      (Rendering|Material|SetMaterial _lights _index "/Game/StarterContent/Materials/M_Glass.M_Glass")
      (else
        (Rendering|Material|SetMaterial _lights (+ _index 1) "/Game/StarterContent/Materials/M_Glass.M_Glass")))))

(fn TurnLighton
  (params (LightIndex :type Integer) (Material :type Material%20Interface%20Object%20Reference))
  (switch int LightIndex
    (:1
      (LocalVariables|SetIndex 0))
    (:2
      (LocalVariables|SetIndex 2))
    (:3
      (LocalVariables|SetIndex 3))
    (:4
      (LocalVariables|SetIndex 4))
    (:5
      (LocalVariables|SetIndex 5))
    (:6
      (LocalVariables|SetIndex 6))
    (:7
      (LocalVariables|SetIndex 7))
    (:8
      (LocalVariables|SetIndex 8))
    (:9
      (LocalVariables|SetIndex 9)))
  (Rendering|Material|SetMaterial (Variables|Default|GetLights) (LocalVariables|GetIndex) Material))

(fn GoThroughSequenceFct
  (bind _level (Variables|Default|GetLevel))
  (bind _sequence (Utilities|Struct|BreakSTR_LightboardLevel _level))
  (bind _returnvalue (Utilities|String|GetCharacterArrayfromString _sequence))
  (if (> (+ (* (Variables|Default|GetStringIndex) 2) 1) (Utilities|Array|LastIndex _returnvalue))
    (CallFunction|TurnLightsOff)
    (Variables|Default|SetbAwaitingInput true)
    (Utilities|Time|ClearandInvalidateTimerbyHandle (Variables|Default|GetTimerHandle))
    (Variables|Default|SetStringIndex 0)
    (else
      (CallFunction|TurnLightsOff)
      (switch string (Utilities|Array|Get(acopy) _returnvalue (+ (* (Variables|Default|GetStringIndex) 2) 1))
        (:g
          (CallFunction|TurnLighton (Math|Conversions|ToInteger(Byte) (Utilities|Array|Get(acopy) _returnvalue (* (Variables|Default|GetStringIndex) 2))) "/Game/Assets/WireBoard/Material/LED_ON.LED_ON"))
        (:b
          (CallFunction|TurnLighton (Math|Conversions|ToInteger(Byte) (Utilities|Array|Get(acopy) _returnvalue (* (Variables|Default|GetStringIndex) 2))) "/Game/Assets/LightBoard/Materials/LED_Blue.LED_Blue"))
        (:r
          (CallFunction|TurnLighton (Math|Conversions|ToInteger(Byte) (Utilities|Array|Get(acopy) _returnvalue (* (Variables|Default|GetStringIndex) 2))) "/Game/Assets/LightBoard/Materials/LED_Red.LED_Red"))
        (:y
          (CallFunction|TurnLighton (Math|Conversions|ToInteger(Byte) (Utilities|Array|Get(acopy) _returnvalue (* (Variables|Default|GetStringIndex) 2))) "/Game/Assets/LightBoard/Materials/LED_Yellow.LED_Yellow")))
      (Variables|Default|SetStringIndex (+ (Variables|Default|GetStringIndex) 1)))))