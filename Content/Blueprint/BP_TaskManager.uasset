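; BP_TaskManager runs the game's overall countdown and starts the lightboard task.
; BeginPlay caches the camera actor, lightboard and wireboard found in the level, then shows the counter widget.
; Tick decrements the time, adding a game-over widget every frame once it runs out.
; Tick also polls the camera's current target to enable the lightboard's timer once; the wireboard reference is unused here.
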(event EventBeginPlay
  (Variables|Default|SettimeRemaining (Variables|Default|GetTotalTime))
  (bind _outactors (Actor|GetAllActorsOfClass "/Game/Blueprint/CameraActor_Blueprint.CameraActor_Blueprint_C"))
  (Variables|Default|SetcamActor (Utilities|Array|Get(acopy) _outactors))
  (bind _outactors_2 (Actor|GetAllActorsOfClass "/Game/Blueprint/BP_Lightboard.BP_Lightboard_C"))
  (Variables|Default|SetlightBoard (Utilities|Array|Get(acopy) _outactors_2))
  (bind _outactors_3 (Actor|GetAllActorsOfClass "/Game/Blueprint/BP_Wireboard.BP_Wireboard_C"))
  (Variables|Default|SetwireBoard (Utilities|Array|Get(acopy) _outactors_3))
  (bind _returnvalue (UserInterface|CreateWidget "/Game/UI/WID_Counter.WID_Counter_C" (Game|GetPlayerController 0)))
  (UserInterface|Viewport|AddtoViewport _returnvalue 0))

(event Collision|EventActorBeginOverlap
  (params (OtherActor :type Actor%20Object%20Reference)))

(event EventTick
  (params (DeltaSeconds :type Float%20%28single-precision%29))
  (bind _lightboard (Variables|Default|GetlightBoard))
  (bind _output_get (Variables|Default|SettimeRemaining (- (Variables|Default|GettimeRemaining) DeltaSeconds)))
  (if (<= _output_get 0.0)
    (bind _returnvalue (UserInterface|CreateWidget "/Game/UI/WID_GAMEOVR.WID_GAMEOVR_C" (Game|GetPlayerController 0)))
    (UserInterface|Viewport|AddtoViewport _returnvalue 0)
    (Variables|Default|SettimeRemaining 0.0))
  (if (and (== (Variables|/Game/Blueprint/CameraActor_Blueprint.CameraActor_Blueprint_C|GetcurrentTarget (Variables|Default|GetcamActor)) 1) (not (Variables|/Game/Blueprint/BP_Lightboard.BP_Lightboard_C|GetActivated (Variables|Default|GetlightBoard))))
    (Default|EnableTimer _lightboard)
    (Variables|/Game/Blueprint/BP_Lightboard.BP_Lightboard_C|SetActivated _lightboard true)))

(fn ConstructionScript)